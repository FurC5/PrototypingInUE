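; Launchpad Blueprint whose Launch event animates its static mesh rising, with no logic here that moves the player or other objects.
; It stores the pad's start location, then LaunchTimeline lerps the mesh toward 30 units above its current position each update, so the rise compounds.
; Each update also plays a second timeline, Delay, whose event track snaps the mesh back to the stored location.
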(event EventLaunch
  (bind _staticmeshcomponent (Variables|Debug|GetStaticMeshComponent))
  (bind _returnvalue (Transformation|GetWorldLocation _staticmeshcomponent))
  (Variables|Default|SetPadLoc (Transformation|GetWorldLocation (Variables|Debug|GetStaticMeshComponent)))
  (bind _launch (Timeline|LaunchTimeline Play)
    (:Update
      (Transformation|SetWorldLocation (Variables|Debug|GetStaticMeshComponent) (Math|Vector|Lerp(Vector) _returnvalue (+ _returnvalue "0, 0,30.000000") _launch) false false)
      (Timeline|delay Play
        (:NewTrack_0
          (Transformation|SetWorldLocation (Variables|Debug|GetStaticMeshComponent) (Variables|Default|GetPadLoc) false false))))))

(fn ConstructionScript)