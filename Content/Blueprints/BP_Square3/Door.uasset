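; Door Blueprint that opens by rising once both the red and blue spheres are in their correct spots.
; External callers set the two flags through SetRedTrue and SetBlueTrue, and ButtontoDoor checks both before playing the DoorOpen timeline.
; Each timeline update lerps the mesh from its current location toward a small upward offset, so movement accumulates rather than interpolating between fixed endpoints.
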(event EventSetRedTrue
  ;[1 1 1] Set the bools to true
  (Variables|Default|SetRedIn? true))

(event EventSetBlueTrue
  ;[1 1 1] Set the bools to true
  (Variables|Default|SetBlueIn? true))

(event EventButtontoDoor
  ;[1 1 1] If both spheres are put in the correct spot then open door
  (if (and (Variables|Default|GetRedIn?) (Variables|Default|GetBlueIn?))
    (bind _newtrack_0 (Timeline|DoorOpen Play)
      (:Update
        (Transformation|SetWorldLocation (Variables|Debug|GetStaticMeshComponent) (Math|Vector|Lerp(Vector) (Transformation|GetWorldLocation (Variables|Debug|GetStaticMeshComponent)) (+ (Transformation|GetWorldLocation (Variables|Debug|GetStaticMeshComponent)) "0,0.000000,3.000000") _newtrack_0) false false)))))

(fn ConstructionScript)