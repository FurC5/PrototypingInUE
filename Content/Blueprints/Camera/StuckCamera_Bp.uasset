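; StuckCamera_Bp is a trigger volume that switches the player's view to a referenced camera while the character is inside its Box.
; On begin overlap, any actor implementing CharacterRef_Interface makes player controller 0 set its view target to CameraRef.
; On end overlap, the same interface check returns the view to CharacterRef.
; The interface only filters actors, and neither reference is assigned in these graphs.
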(event OnComponentBeginOverlap(Box)
  (params (OverlappedComponent :type Primitive%20Component%20Object%20Reference) (OtherActor :type Actor%20Object%20Reference) (OtherComp :type Primitive%20Component%20Object%20Reference) (OtherBodyIndex :type Integer) (bFromSweep :type Boolean) (SweepResult :type Hit%20Result%20Structure%20%28by%20ref%29))
  (if (Utilities|DoesObjectImplementInterface OtherActor "/Game/Blueprints/Camera/CharacterRef_Interface.CharacterRef_Interface_C")
    (Game|Player|SetViewTargetwithBlend (Game|GetPlayerController 0) (Variables|Default|GetCamera_Ref) 0.0 "VTBlend_Linear" 0.0 false)))

(event OnComponentEndOverlap(Box)
  (params (OverlappedComponent :type Primitive%20Component%20Object%20Reference) (OtherActor :type Actor%20Object%20Reference) (OtherComp :type Primitive%20Component%20Object%20Reference) (OtherBodyIndex :type Integer))
  (if (Utilities|DoesObjectImplementInterface OtherActor "/Game/Blueprints/Camera/CharacterRef_Interface.CharacterRef_Interface_C")
    (Game|Player|SetViewTargetwithBlend (Game|GetPlayerController 0) (Variables|Default|GetCharacterRef) 0.0 "VTBlend_Linear" 0.0 false)))

(fn ConstructionScript)