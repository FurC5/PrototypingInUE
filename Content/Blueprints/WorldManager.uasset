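; WorldManager builds the world at runtime from randomly chosen streaming sublevel tiles.
; BeginGeneration loops over the grid size, drawing names from SquareName without repeats, then instances each level and sets it loaded and visible.
; Each instance's X location comes from the Math helper, whose centering formula appears unconnected in its graph.
; Random 90-degree rotation and a second-axis loop exist but are unused.
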(event EventBeginGeneration
  (for _index (range 0 (Variables|Default|GetLevelGridSize))
    (bind _returnvalue (CallFunction|StreamChunk/RemovefromList))
    (bind _returnvalue_2 (Class|LevelStreaming|CreateInstance _returnvalue (Utilities|String|ToString(Integer) _index)))
    (Utilities|Array|Clear (Variables|Default|GetRemoveList))
    (Variables|/Script/Engine.LevelStreaming|SetLevelTransform _returnvalue_2 (Math|Transform|MakeTransform (Math|Vector|MakeVector (Utilities|Math _index (/ (* (Variables|Default|GetLevelGridSize) (Variables|Default|GetTileSize)) 2.0)) 0.0 0.0)))
    (Variables|/Script/Engine.LevelStreaming|SetbShouldBeLoaded _returnvalue_2 true)
    (Variables|/Script/Engine.LevelStreaming|SetbShouldBeVisible _returnvalue_2 true)))

(fn ConstructionScript)

(fn GetRandomRotation
  (return (* (Math|Random|RandomInteger 4) 9e+01)))

(fn GetRandomIntance
  (bind _squarename (Variables|Default|GetSquareName))
  (return (Utilities|Array|Get(acopy) _squarename (Math|Random|RandomInteger (Utilities|Array|Length _squarename)))))

(fn StreamChunk/RemovefromList
  (bind _returnvalue (Utilities|Array|Add (Variables|Default|GetRemoveList) (CallFunction|GetRandomIntance)))
  (Utilities|Array|RemoveItem (Variables|Default|GetSquareName) (Utilities|Array|Get(acopy) (Variables|Default|GetRemoveList) _returnvalue))
  (return (Class|GameplayStatics|GetStreamingLevel (Utilities|Array|Get(acopy) (Variables|Default|GetRemoveList) _returnvalue))))