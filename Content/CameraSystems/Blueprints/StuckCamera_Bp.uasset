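; StuckCamera_Bp is a camera trigger volume that switches the player's view to a referenced camera while a character is inside its box.
; On begin overlap, any actor implementing CharacterRef_Interface makes player controller 0 blend its view target to CameraRef over BlendTime.
; On end overlap, the same check blends the view back to the player character.
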(event OnComponentBeginOverlap(Box)
  (params (OverlappedComponent :type Primitive%20Component%20Object%20Reference) (OtherActor :type Actor%20Object%20Reference) (OtherComp :type Primitive%20Component%20Object%20Reference) (OtherBodyIndex :type Integer) (bFromSweep :type Boolean) (SweepResult :type Hit%20Result%20Structure%20%28by%20ref%29))
  (if (Utilities|DoesObjectImplementInterface OtherActor "/Game/SplineSystems(NOT_USED)/TestDude/CharacterRef_Interface.CharacterRef_Interface_C")
    (Game|Player|SetViewTargetwithBlend (Game|GetPlayerController 0) (Variables|Default|GetCamera_Ref) (Variables|Default|GetBlendTime) "VTBlend_Linear" 0.0 false)))

(event OnComponentEndOverlap(Box)
  (params (OverlappedComponent :type Primitive%20Component%20Object%20Reference) (OtherActor :type Actor%20Object%20Reference) (OtherComp :type Primitive%20Component%20Object%20Reference) (OtherBodyIndex :type Integer))
  (if (Utilities|DoesObjectImplementInterface OtherActor "/Game/SplineSystems(NOT_USED)/TestDude/CharacterRef_Interface.CharacterRef_Interface_C")
    (Game|Player|SetViewTargetwithBlend (Game|GetPlayerController 0) (Game|GetPlayerCharacter 0) (Variables|Default|GetBlendTime) "VTBlend_Linear" 0.0 false)))

(fn ConstructionScript)