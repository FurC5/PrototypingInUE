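; Spline movement component, in a folder marked not used, that confines its owning actor to a path spline and drives a spline-based camera.
; UpdatePlayer clamps the owner's offset from the nearest path point in 2D, using PathWidth times the spline's Y scale.
; It places the camera on CameraSpline, either nearest the target or at the path's matching input key, aims it at the target and matches control rotation.
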(event Custom|UpdatePlayer
  (bind _returnvalue (Components|GetOwner))
  (bind _returnvalue_2 (Components|GetOwner))
  (bind _pathspline (Variables|Default|GetPathSpline))
  (bind _cameraspline (Variables|Default|GetCameraSpline))
  (bind _uselocationbasedcamera (Variables|Default|GetUseLocationBasedCamera))
  (bind _returnvalue_3 (Components|GetOwner _returnvalue))
  (bind _returnvalue_4 (Transformation|GetActorLocation _returnvalue_2))
  (bind _returnvalue_5 (Transformation|GetActorLocation _returnvalue_3))
  (bind _returnvalue_6 (Class|SplineComponent|FindInputKeyClosesttoWorldLocation _pathspline _returnvalue_4))
  (bind (_returnvalue_7 _returnvalue2) (CallFunction|GetNearestSplineRotation _cameraspline _returnvalue_5))
  (bind (_returnvalue_8 _returnvalue2_2) (CallFunction|GetKeyRelativeLocation _returnvalue_5 _cameraspline _returnvalue_6))
  (bind _returnvalue_9 (select _uselocationbasedcamera _returnvalue2 _returnvalue_8))
  (if (and (Utilities|IsValid (Variables|Default|GetPathSpline)) (Utilities|IsValid (Variables|Default|GetCameraSpline)))
    (Transformation|SetActorLocation (Components|GetOwner) (CallFunction|GetSplineScaledPosition _returnvalue_2 _pathspline) false false)
    (bind _camera (Class|ComponentInterface|GetCamera(Message) _returnvalue))
    (Utilities|IsValid _camera
      (:Is%20Valid
        (Transformation|SetWorldLocationAndRotation _camera (select (Variables|Default|GetUseLocationBasedCamera) _returnvalue_7 _returnvalue2_2) _returnvalue_9 false false)
        (Pawn|SetControlRotation (Game|GetPlayerController 0) _returnvalue_9)))))

(fn GetSplineScaledPosition
  (params (InputPin :type Actor%20Object%20Reference) (InputPin2 :type Spline%20Component%20Object%20Reference))
  (bind _returnvalue (Transformation|GetActorLocation InputPin))
  (bind _pathwidth (Variables|Default|GetPathWidth))
  (bind _returnvalue_2 (Spline|FindLocationClosesttoWorldLocation InputPin2 _returnvalue "World"))
  (bind _returnvalue_3 (Class|SplineComponent|FindScaleClosesttoWorldLocation InputPin2 _returnvalue))
  (bind _returnvalue_4 (* _pathwidth (.y _returnvalue_3)))
  (return (+ _returnvalue_2 (Math|Vector|VectorClampSize2D (- (Transformation|GetActorLocation InputPin) _returnvalue_2) (* _returnvalue_4 -1.0) _returnvalue_4))))

(fn GetNearestSplineRotation
  (params (self2 :type Spline%20Component%20Object%20Reference) (InputPin :type Vector))
  (bind _returnvalue (Spline|FindLocationClosesttoWorldLocation self2 InputPin "World"))
  (return _returnvalue (Math|Rotator|FindLookatRotation _returnvalue InputPin)))

(fn GetKeyRelativeLocation
  (params (Target :type Vector%20%28by%20ref%29) (self2 :type Spline%20Component%20Object%20Reference) (InKey :type Float%20%28single-precision%29))
  (bind _returnvalue (Class|SplineComponent|GetLocationatSplineInputKey self2 InKey "World"))
  (return (Math|Rotator|FindLookatRotation _returnvalue Target) _returnvalue))