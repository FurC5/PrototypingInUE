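; TrackSwitch is a trigger-box actor that switches overlapping actors onto new path and camera splines, in a folder marked as not used.
; On begin overlap it sends the character an entered-switch message, then passes the overlapping actor the splines from its referenced path and camera actors, if both are valid.
; Shortly after BeginPlay it also hands those splines to actors already inside the box, without the entered-switch message.
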(event OnComponentBeginOverlap(Box)
  (params (OverlappedComponent :type Primitive%20Component%20Object%20Reference) (OtherActor :type Actor%20Object%20Reference) (OtherComp :type Primitive%20Component%20Object%20Reference) (OtherBodyIndex :type Integer) (bFromSweep :type Boolean) (SweepResult :type Hit%20Result%20Structure%20%28by%20ref%29))
  (Class|EnteredTrackSwitchInterface|EnteredTrackSwitch(Message) (Variables|Default|GetCharacter))
  (if (and (Utilities|IsValid (Variables|Default|GetPathActorRef)) (Utilities|IsValid (Variables|Default|GetCameraActorRef)))
    (bind _spline (Class|SplineInterface|GetSpline(Message) (Variables|Default|GetCameraActorRef)))
    (Class|ComponentInterface|SetCameraSpline(Message) OtherActor _spline)
    (bind _spline_2 (Class|SplineInterface|GetSpline(Message) (Variables|Default|GetPathActorRef)))
    (Class|ComponentInterface|SetPathSpline(Message) OtherActor _spline_2)))

(event EventBeginPlay
  (Utilities|FlowControl|Delay 0.2)
  (for _array_element (Collision|GetOverlappingActors (Variables|Default|GetBox) 0 :!class /Script/Engine.PrimitiveComponent)
    (if (and (Utilities|IsValid (Variables|Default|GetPathActorRef)) (Utilities|IsValid (Variables|Default|GetCameraActorRef)))
      (bind _spline (Class|SplineInterface|GetSpline(Message) (Variables|Default|GetCameraActorRef)))
      (Class|ComponentInterface|SetCameraSpline(Message) _array_element _spline)
      (bind _spline_2 (Class|SplineInterface|GetSpline(Message) (Variables|Default|GetPathActorRef)))
      (Class|ComponentInterface|SetPathSpline(Message) _array_element _spline_2))))

(fn ConstructionScript)